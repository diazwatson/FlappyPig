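; BP_Obstacle is a moving obstacle that carries a Bean component worth a point.
; On BeginPlay it shifts its root to a random height within a fixed Z range, then moves it along X every Tick at Speed, scaled by delta time.
; When anything begins overlapping the Bean, it calls AddPoint on BP_GameMode, plays the Point sound and destroys the Bean component.
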(event OnComponentBeginOverlap(Bean)
  (params (OverlappedComponent :type Primitive%20Component%20Object%20Reference) (OtherActor :type Actor%20Object%20Reference) (OtherComp :type Primitive%20Component%20Object%20Reference) (OtherBodyIndex :type Integer) (bFromSweep :type Boolean) (SweepResult :type Hit%20Result%20Structure%20%28by%20ref%29))
  ;[0.3252 1 0.3114] Add Point
  (bind _asbp_game_mode (Utilities|Casting|CastToBP_GameMode (Game|GetGameMode)))
  (Default|AddPoint _asbp_game_mode)
  (Audio|PlaySound2D "/Game/Audio/point.point" 1.0 1.0 0.0 0 0)
  (Components|DestroyComponent (Variables|Default|GetBean)))

(event EventBeginPlay
  (bind _defaultsceneroot (Variables|Default|GetDefaultSceneRoot))
  (bind _returnvalue (Transformation|GetWorldLocation _defaultsceneroot))
  (Transformation|SetWorldLocation _defaultsceneroot (Math|Vector|MakeVector (.x _returnvalue) (.y _returnvalue) (Math|Random|RandomFloatinRange -7e+01 7e+01)) false false))

(event Collision|EventActorBeginOverlap
  (params (OtherActor :type Actor%20Object%20Reference)))

(event EventTick
  (params (DeltaSeconds :type Float%20%28single-precision%29))
  (Transformation|SetWorldLocation (Variables|Default|GetDefaultSceneRoot) (+ (Transformation|GetWorldLocation (Variables|Default|GetDefaultSceneRoot)) (Math|Vector|MakeVector (* DeltaSeconds (Math|Float|MakeLiteralFloat (Variables|Default|GetSpeed))) 0.0 0.0)) false false))

(fn ConstructionScript)