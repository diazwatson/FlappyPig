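; BP_ObstableSpawner is an actor that spawns obstacles at its own root transform while the player character is playing.
; BeginPlay caches the player pawn as BP_Character, printing a message if the cast fails.
; Tick checks IsPlaying and runs a random Delay, which ignores re-triggers while pending and so paces spawns at irregular intervals.
; Each spawned obstacle gets a fixed lifespan so it cleans itself up.
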(event EventBeginPlay
  (bind _asbp_character (Utilities|Casting|CastToBP_Character (Game|Player|GetPlayerPawn 0))
    (:then
      (Variables|Default|SetPlayer _asbp_character))
    (:CastFailed
      (Development|PrintString "Failing to Cast BP_Character"))))

(event Collision|EventActorBeginOverlap
  (params (OtherActor :type Actor%20Object%20Reference)))

(event EventTick
  (params (DeltaSeconds :type Float%20%28single-precision%29))
  (if (Variables|/Game/Blueprints/BP_Character.BP_Character_C|GetIsPlaying (Variables|Default|GetPlayer))
    (Utilities|FlowControl|Delay (Math|Random|RandomFloatinRange 1.5 5.0))
    (bind _returnvalue (Game|SpawnActorfromClass "/Game/Blueprints/BP_Obstacle.BP_Obstacle_C" (Transformation|GetWorldTransform (Variables|Default|GetDefaultSceneRoot)) "Undefined" 0 0))
    (Actor|SetLifeSpan _returnvalue 1e+01)))

(fn ConstructionScript)