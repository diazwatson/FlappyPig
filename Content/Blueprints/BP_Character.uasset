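; Player pawn for a one-button, Flappy Bird-style game: a physics capsule with a Paper2D sprite that jumps with fart sounds.
; The first press enables gravity; each jump resets velocity, applies an upward impulse and briefly swaps the sprite.
; While rising, extra downward force is lighter with Jump held, allowing variable height.
; Overlapping "Enemy"-tagged components kills it with a spin and sounds, then restarts Main on a press or timeout.
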(event OnComponentBeginOverlap(Capsule)
  (params (OverlappedComponent :type Primitive%20Component%20Object%20Reference) (OtherActor :type Actor%20Object%20Reference) (OtherComp :type Primitive%20Component%20Object%20Reference) (OtherBodyIndex :type Integer) (bFromSweep :type Boolean) (SweepResult :type Hit%20Result%20Structure%20%28by%20ref%29))
  (Utilities|IsValid OtherComp
    (:Is%20Valid
      (if (Components|ComponentHasTag OtherComp "Enemy")
        ;[1 0.5117 0.5043] Death
        (if (Variables|Default|GetIsAlive)
          (Variables|Default|SetIsAlive false)
          (CallFunction|Jump)
          (Class|PrimitiveComponent|AddTorqueinDegrees (Variables|Default|GetCapsule) "0.0,-100000.000000,0.0" "None" true)
          (Audio|SpawnSound2D "/Game/Audio/game_over.game_over" 1.0 1.0 0.0 0)
          (Audio|SpawnSound2D "/Game/Audio/FartDie.FartDie" 5.0 1.0 0.0 0)
          (Utilities|FlowControl|Delay 3.0)
          (Variables|Default|SetReadyToRestart true)
          (Utilities|FlowControl|Delay 3.0)
          (CallFunction|RestartLevel))))))

(event EventBeginPlay
  (Physics|SetEnableGravity (Variables|Default|GetCapsule) false))

(event EventTick
  (params (DeltaSeconds :type Float%20%28single-precision%29))
  ;[1 1 1] Modified Gravity for Jump
  (bind _returnvalue (Physics|GetPhysicsLinearVelocity (Variables|Default|GetCapsule) "None"))
  (if (> (.z _returnvalue) 0.0)
    (if (== (Input|AxisValues|GetJump) 1.0)
      (Variables|Default|SetDownForce -5e+01)
      (else
        (Variables|Default|SetDownForce -1e+02)))
    (Physics|AddForce (Variables|Default|GetCapsule) (Math|Vector|MakeVector 0.0 0.0 (Variables|Default|GetDownForce)) "None" false)))

(event Input|ActionEvents|InputActionJump
  (params (Key :type Key%20Structure :default "None"))
  (:Pressed
    (Rendering|Components|Sprite|SetSprite (Variables|Default|GetPaperSprite) "/Game/Sprites/SpriteSheet3_Sprite_1.SpriteSheet3_Sprite_1")
    (Utilities|FlowControl|Delay 0.5)
    (Rendering|Components|Sprite|SetSprite (Variables|Default|GetPaperSprite) "/Game/Sprites/SpriteSheet3_Sprite_0.SpriteSheet3_Sprite_0")))

(event Input|ActionEvents|InputActionJump
  (params (Key :type Key%20Structure :default "None"))
  (bind _returnvalue (Game|GetPlayerController 0))
  (:Pressed
    ;[1 1 1] Jump Mechanics
    (if (Variables|Default|GetIsPlaying)
      _
      (else
        (Variables|Default|SetIsPlaying true)
        (Physics|SetEnableGravity (Variables|Default|GetCapsule) true)))
    (if (Variables|Default|GetIsAlive)
      (CallFunction|Jump)
      (Audio|PlaySound2D "/Game/Audio/Fart.Fart" 1.0 1.0 0.0 0 0)
      (Game|Feedback|ClientPlayForceFeedback _returnvalue "/Game/ForceFeedbackEffect.ForceFeedbackEffect" "None" false false false)
      (Game|Feedback|PlayDynamicForceFeedback _returnvalue 0.0 -1.0 true true true true)
      (elif (Variables|Default|GetReadyToRestart)
        (Game|OpenLevel(byName) "Main")))))

(event Input|KeyboardEvents|Escape
  (params (Key :type Key%20Structure :default "None"))
  (:Pressed
    (Game|QuitGame 0 "Quit" false)))

(event Input|GamepadEvents|GamepadSpecialLeft
  (params (Key :type Key%20Structure :default "None"))
  (:Pressed
    (CallFunction|RestartLevel)))

(fn ConstructionScript)

(fn Jump
  (Physics|SetPhysicsLinearVelocity (Variables|Default|GetCapsule) "0, 0, 0" false "None")
  (Physics|AddImpulse (Variables|Default|GetCapsule) "0, 0,25.000000" "None" false))

(fn RestartLevel
  (Game|OpenLevel(byName) "Main"))