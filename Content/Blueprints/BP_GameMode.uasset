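; BP_GameMode is a game mode that handles music, score and the score HUD.
; On BeginPlay it casts the player pawn to BP_Character, starts 2D music and adds a ScoreInterface widget to the viewport.
; Tick polls the player's IsAlive flag and stops the music once the player is dead.
; AddPoint increments the Score variable.
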(event EventTick
  (params (DeltaSeconds :type Float%20%28single-precision%29))
  (bind _music (Variables|Default|GetMusic))
  (if (not (Variables|/Game/Blueprints/BP_Character.BP_Character_C|GetIsAlive (Variables|Default|GetPlayer)))
    (Utilities|IsValid _music
      (:Is%20Valid
        (Audio|Components|Audio|Stop _music)))))

(event EventBeginPlay
  (bind _asbp_character (Utilities|Casting|CastToBP_Character (Game|Player|GetPlayerPawn 0))
    (:then
      (Variables|Default|SetPlayer _asbp_character)
      (bind _returnvalue (Audio|SpawnSound2D "/Game/Audio/Music.Music" 1.0 1.0 0.0 0))
      (Variables|Default|SetMusic _returnvalue)
      (bind _returnvalue_2 (UserInterface|CreateWidget "/Game/UI/ScoreInterface.ScoreInterface_C"))
      (UserInterface|Viewport|AddtoViewport _returnvalue_2 0))
    (:CastFailed
      (Development|PrintString "Failing to Cast BP_Character"))))

(fn ConstructionScript)

(fn AddPoint
  (Math|Integer|IncrementInt (Variables|Default|GetScore)))